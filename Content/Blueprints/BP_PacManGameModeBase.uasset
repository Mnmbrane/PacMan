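; Game mode Blueprint for a Pac-Man game that tracks elapsed time and holds the current ghost mode, Scatter or Chase.
; On BeginPlay it starts a looping one-second timer that increments the time counter and prints it alongside the ghost mode as on-screen debug text.
; A getter exposes the ghost mode, and a helper converts it to a string; nothing in this graph changes the mode.
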(event `self.ReceiveBeginPlay`
  (`self.Start Print Time Handler`))

(event `Start Print Time Handler`
  ;[1 1 1] Print Time
  (`KismetSystemLibrary.K2_SetTimerDelegate` (delegate `PrintTime`) 1.0 true))

(event `PrintTime`
  ;[1 1 1] Print Time
  (bind _output_get (set `self.mTimeCounter` (+ (`self.mTimeCounter`) 1.0)))
  (`KismetSystemLibrary.PrintString` (`KismetTextLibrary.Conv_TextToString` (`|FormatText` "Time: {time}" (`KismetStringLibrary.Conv_DoubleToString` _output_get))) true true (struct :`G` 0.66 :`B` 1.0 :`A` 1.0) 1.0)
  ;[1 1 1] Print Ghost Mode
  (bind _retstring (`self.GetStringFromGhostMode`))
  (`KismetSystemLibrary.PrintString` (`KismetTextLibrary.Conv_TextToString` (`|FormatText` "Current Ghost Mode: {mode}" _retstring)) true true (struct :`G` 0.66 :`B` 1.0 :`A` 1.0) 1.0))

(fn `GetGhostMode`
  (returns (GhostMode :type Byte))
  (return (`self.mGhostMode`)))

(fn `GetStringFromGhostMode`
  (returns (retString :type String))
  (switch `|SwitchEnum` (`self.mGhostMode`)
    (:`NewEnumerator0`
      (return "Scatter"))
    (:`NewEnumerator1`
      (return "Chase"))))

(fn `UserConstructionScript`)